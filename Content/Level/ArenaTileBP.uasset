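; Base Blueprint for an arena tile that takes damage and regenerates health after a delay.
; AnyDamage subtracts health, then either calls destruction or resets the regen timer, and calls particle, sound and material color hooks.
; Tick counts up to the regen delay, then restores health at a set rate, clamped to max, refreshing the color.
; Destruction, particle, sound and color handlers are empty stubs.
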(event EventBeginPlay)

(event Collision|EventActorBeginOverlap
  (params (OtherActor :type Actor%20Object%20Reference)))

(event EventTick
  (params (DeltaSeconds :type Float%20%28single-precision%29))
  (CallFunction|HandleRegenHealth DeltaSeconds))

(event Game|Damage|EventAnyDamage
  (params (Damage :type Float%20%28single-precision%29) (DamageType :type Damage%20Type%20Object%20Reference) (InstigatedBy :type Controller%20Object%20Reference) (DamageCauser :type Actor%20Object%20Reference))
  ;[1 1 1] Tile Takes Damage
  (CallFunction|HandleDamagetoHealth Damage DamageType InstigatedBy DamageCauser)
  (CallFunction|HandleDamageParticles Damage DamageType InstigatedBy DamageCauser)
  (CallFunction|HandleDamageSound Damage DamageType InstigatedBy DamageCauser)
  (CallFunction|HandleMaterialColorChange))

(fn ConstructionScript
  (Variables|Default|SetCurrentHealth (Variables|Default|GetMaxHealth)))

(fn HandleDamagetoHealth
  (params (Damage :type Float%20%28single-precision%29) (DamageType :type Damage%20Type%20Object%20Reference) (InstigatedBy :type Controller%20Object%20Reference) (DamageCauser :type Actor%20Object%20Reference))
  (bind _output_get (Variables|Default|SetCurrentHealth (- (Variables|Default|GetCurrentHealth) Damage)))
  (if (<= _output_get 0.0)
    (CallFunction|HandleDestruction Damage DamageType InstigatedBy DamageCauser)
    (else
      (CallFunction|ResetRegenTimer))))

(fn HandleDestruction
  (params (Damage :type Float%20%28single-precision%29) (Damage%20Type :type Damage%20Type%20Object%20Reference) (InstigatedBy :type Controller%20Object%20Reference) (DamageCauser :type Actor%20Object%20Reference)))

(fn HandleDamageParticles
  (params (Damage :type Float%20%28single-precision%29) (DamageType :type Damage%20Type%20Object%20Reference) (InstigatedBy :type Controller%20Object%20Reference) (DamageCauser :type Actor%20Object%20Reference)))

(fn HandleDamageSound
  (params (Damage :type Float%20%28single-precision%29) (DamageType :type Damage%20Type%20Object%20Reference) (InstigatedBy :type Controller%20Object%20Reference) (DamageCauser :type Actor%20Object%20Reference)))

(fn HandleMaterialColorChange)

(fn ResetRegenTimer
  (Variables|Default|SetcanRegen false)
  (Variables|Default|SetHealthRegenTimerElapsed 0.0))

(fn HandleRegenHealth
  (params (DeltaSeconds :type Float%20%28single-precision%29))
  (bind _maxhealth (Variables|Default|GetMaxHealth))
  (if (Variables|Default|GetcanRegen)
    (Variables|Default|SetCurrentHealth (Math|Float|MapRangeClamped (+ (Variables|Default|GetCurrentHealth) (* (Variables|Default|GetHealthRegenRate) DeltaSeconds)) 0.0 _maxhealth 0.0 _maxhealth) :!label _label)
    (CallFunction|HandleMaterialColorChange)
    (elif (>= (Variables|Default|GetHealthRegenTimerElapsed) (Variables|Default|GetHealthRegenDelay))
      (Variables|Default|SetcanRegen true)
      (goto _label)
      (else
        (CallFunction|UpdateRegenTimer DeltaSeconds)))))

(fn UpdateRegenTimer
  (params (DeltaSeconds :type Float%20%28single-precision%29))
  (Variables|Default|SetHealthRegenTimerElapsed (+ DeltaSeconds (Variables|Default|GetHealthRegenTimerElapsed))))
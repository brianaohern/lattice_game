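; Arena Blueprint that procedurally builds a level from tiles and player starts when StartBuild receives X, Y and Z dimensions.
; Nested loops spawn ArenaTileBP actors in a 3D grid, then LatticePlayerStarts spawn for a hardcoded player count.
; Free-for-all starts use sine/cosine to form an inset ellipse, rotated toward the arena center.
; The team-game branch places every start at the same origin-corner XY position.
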(event EventBeginPlay)

(event Collision|EventActorBeginOverlap
  (params (OtherActor :type Actor%20Object%20Reference)))

(event EventTick
  (params (DeltaSeconds :type Float%20%28single-precision%29)))

(event EventStartBuild
  (params (x :type Integer) (y :type Integer) (z :type Integer))
  (bind _returnvalue (- y 1))
  (bind _returnvalue_2 (- x 1))
  (bind _tilesize (Variables|Default|GetTileSize))
  (bind _tilesize_2 (Variables|Default|GetTileSize))
  (bind _tilesize_3 (Variables|Default|GetTileSize))
  (bind _returnvalue_3 (* _returnvalue _tilesize_2))
  (bind _returnvalue_4 (* _returnvalue_2 _tilesize_3))
  (bind _returnvalue_5 (/ _returnvalue_3 2))
  (bind _returnvalue_6 (/ _returnvalue_4 2))
  ;[1 1 1] Build Tiles
  (for _index (range 0 _returnvalue_2)
    (for _index_2 (range 0 _returnvalue)
      (for _index_3 (range 0 (- z 1))
        (Game|SpawnActorfromClass "/Game/Level/ArenaTileBP.ArenaTileBP_C" (Math|Transform|MakeTransform (Math|Vector|MakeVector (Math|Conversions|ToFloat(Integer) (* _index _tilesize)) (Math|Conversions|ToFloat(Integer) (* _index_2 _tilesize)) (Math|Conversions|ToFloat(Integer) (* _index_3 (Variables|Default|GetTileHeight))))) "Undefined" 0 0))))
  ;[1 1 1] Build Player Starts
  (bind _output_get (Variables|Default|SetArenaCenter (Math|Vector|MakeVector (Math|Conversions|ToFloat(Integer) _returnvalue_6) (Math|Conversions|ToFloat(Integer) _returnvalue_5) (Math|Conversions|ToFloat(Integer) (Variables|Default|GetTileHeight)))))
  (bind _player_count (CallFunction|GetPlayerCount))
  (bind _output_get_2 (Variables|Default|SetPlayerCount _player_count))
  (for _index_4 (range 0 (- _output_get_2 1))
    (if (Variables|Default|GetIsTeamGame)
      (Game|SpawnActorfromClass "/Script/LatticeGame.LatticePlayerStart" (Math|Transform|MakeTransform (Math|Vector|MakeVector 0.0 0.0 (Math|Conversions|ToFloat(Integer) (+ (* (- z 1) 1000) 50))) (Math|Rotator|MakeRotator 0.0 0.0 0.0)) "Undefined" 0 0)
      (else
        ;;[1 1 1] Spawn in a Circle, Facing Inward
        (Game|SpawnActorfromClass "/Script/LatticeGame.LatticePlayerStart" (Math|Transform|MakeTransform (Math|Vector|MakeVector (|((Radius*(sin(theta)))+XCenter) (* (/ (* (Math|Trig|GetPI) 2.0) (Math|Conversions|ToFloat(Integer) (Variables|Default|GetPlayerCount))) (Math|Conversions|ToFloat(Integer) _index_4)) (.X (Math|Vector|BreakVector _output_get)) (Math|Conversions|ToFloat(Integer) (- _returnvalue_6 200))) (|((Radius*(cos(theta)))+YCenter) (* (/ (* (Math|Trig|GetPI) 2.0) (Math|Conversions|ToFloat(Integer) (Variables|Default|GetPlayerCount))) (Math|Conversions|ToFloat(Integer) _index_4)) (Math|Conversions|ToFloat(Integer) (- _returnvalue_5 200)) (.Y (Math|Vector|BreakVector _output_get))) (Math|Conversions|ToFloat(Integer) (+ (* (- z 1) 1000) 75))) (Math|Rotator|FindLookatRotation (Math|Vector|MakeVector (|((Radius*(sin(theta)))+XCenter) (* (/ (* (Math|Trig|GetPI) 2.0) (Math|Conversions|ToFloat(Integer) (Variables|Default|GetPlayerCount))) (Math|Conversions|ToFloat(Integer) _index_4)) (.X (Math|Vector|BreakVector _output_get)) (Math|Conversions|ToFloat(Integer) (- _returnvalue_6 200))) (|((Radius*(cos(theta)))+YCenter) (* (/ (* (Math|Trig|GetPI) 2.0) (Math|Conversions|ToFloat(Integer) (Variables|Default|GetPlayerCount))) (Math|Conversions|ToFloat(Integer) _index_4)) (Math|Conversions|ToFloat(Integer) (- _returnvalue_5 200)) (.Y (Math|Vector|BreakVector _output_get))) (Math|Conversions|ToFloat(Integer) (+ (* (- z 1) 1000) 75))) (Variables|Default|GetArenaCenter))) "Undefined" 0 0)))))

(fn ConstructionScript)

(fn GetPlayerCount
  (return 16))
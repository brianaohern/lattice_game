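; ArenaBP is an actor that builds an arena by spawning a three-dimensional grid of ArenaTileBP tiles.
; Its StartBuild event takes X, Y and Z tile counts and runs nested loops, placing each tile at fixed spacing, with a wider step between vertical layers.
; Tiles spawn at world-space positions measured from the origin, unrotated and at unit scale; nothing in this Blueprint calls StartBuild itself.
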(event EventBeginPlay)

(event Collision|EventActorBeginOverlap
  (params (OtherActor :type Actor%20Object%20Reference)))

(event EventTick
  (params (DeltaSeconds :type Float%20%28single-precision%29)))

(event EventStartBuild
  (params (x :type Integer) (y :type Integer) (z :type Integer))
  (for _index (range 0 (- x 1))
    (for _index_2 (range 0 (- y 1))
      (for _index_3 (range 0 (- z 1))
        (Game|SpawnActorfromClass "/Game/ArenaTileBP.ArenaTileBP_C" (Math|Transform|MakeTransform (Math|Vector|MakeVector (Math|Conversions|ToFloat(Integer) (* _index 400)) (Math|Conversions|ToFloat(Integer) (* _index_2 400)) (Math|Conversions|ToFloat(Integer) (* _index_3 1000)))) "Undefined" 0 0)))))

(fn ConstructionScript)